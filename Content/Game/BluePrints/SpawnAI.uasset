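; SpawnAI is a timed enemy spawner that creates AIennemy pawns at a fixed world location when play begins.
; A Sequence on BeginPlay runs two delayed chains in parallel: a short staggered wave of four weak enemies and a single higher-health enemy later.
; Both chains call the Spawn function, which spawns the AI and sets its current and maximum health (Vie, MaxVie) from the Hp input.
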(event EventBeginPlay
  (Utilities|FlowControl|Sequence
    (:then_0
      (Utilities|FlowControl|Delay 1.5)
      (CallFunction|Spawn 1e+01)
      (Utilities|FlowControl|Delay 1.0)
      (CallFunction|Spawn 1e+01)
      (Utilities|FlowControl|Delay 1.0)
      (CallFunction|Spawn 1e+01)
      (Utilities|FlowControl|Delay 1.0)
      (CallFunction|Spawn 1e+01))
    (:then_1
      (Utilities|FlowControl|Delay 2e+01)
      (CallFunction|Spawn 5e+01))))

(fn ConstructionScript)

(fn Spawn
  (params (Hp :type Float%20%28single-precision%29))
  (bind _returnvalue (AI|SpawnAIFromClass "/Game/Game/BluePrints/AIennemy.AIennemy_C" 0 "-5800.000000,3715.000000,170.000000" "0, 0, 0" false))
  (bind _asaiennemy (Utilities|Casting|CastToAIennemy _returnvalue))
  (Variables|/Game/Game/BluePrints/AIennemy.AIennemy_C|SetVie _asaiennemy Hp)
  (bind _asaiennemy_2 (Utilities|Casting|CastToAIennemy _returnvalue))
  (Variables|/Game/Game/BluePrints/AIennemy.AIennemy_C|SetMaxVie _asaiennemy_2 Hp))