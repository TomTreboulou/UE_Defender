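; Enemy AI pawn that moves to a target point, damaging the player if it arrives and rewarding the player if killed.
; After a short delay it heads for the first TargetPoint found, then destroys itself and calls TakeDamage on My_Camera.
; LooseHp subtracts health, and at zero destroys the enemy, grants money and score, and returns false.
; Tick swaps the sphere's material to show remaining health.
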(event EventBeginPlay
  (Utilities|FlowControl|Delay 0.2)
  (bind _outactors (Actor|GetAllActorsOfClass "/Script/Engine.TargetPoint"))
  (AI|AIMoveTo self "0, 0, 0" (Utilities|Array|Get(acopy) _outactors) 5.0 false
    (:OnSuccess
      (Actor|DestroyActor)
      (bind _asmy_camera (Utilities|Casting|CastToMy_Camera (Game|GetPlayerCharacter 0)))
      (Default|TakeDamage _asmy_camera 0.1))))

(event EventTick
  (params (DeltaSeconds :type Float%20%28single-precision%29))
  (bind _sphere (Variables|Default|GetSphere))
  (switch int (Math|Float|Truncate (Variables|Default|GetVie))
    (:0
      (Rendering|Material|SetMaterial _sphere 0 "/Game/Game/BluePrints/Health/Health1.Health1" :!label _label))
    (:1
      (goto _label))
    (:2
      (Rendering|Material|SetMaterial _sphere 0 "/Game/Game/BluePrints/Health/Health2.Health2"))
    (:3
      (Rendering|Material|SetMaterial _sphere 0 "/Game/Game/BluePrints/Health/Health3.Health3"))
    (:4
      (Rendering|Material|SetMaterial _sphere 0 "/Game/Game/BluePrints/Health/Health4.Health4"))
    (:5
      (Rendering|Material|SetMaterial _sphere 0 "/Game/Game/BluePrints/Health/Health5.Health5"))
    (:6
      (Rendering|Material|SetMaterial _sphere 0 "/Game/Game/BluePrints/Health/Health6.Health6"))
    (:7
      (Rendering|Material|SetMaterial _sphere 0 "/Game/Game/BluePrints/Health/Health7.Health7"))
    (:8
      (Rendering|Material|SetMaterial _sphere 0 "/Game/Game/BluePrints/Health/Health8.Health8"))
    (:9
      (Rendering|Material|SetMaterial _sphere 0 "/Game/Game/BluePrints/Health/Health9.Health9"))
    (:10
      (Rendering|Material|SetMaterial _sphere 0 "/Game/Game/BluePrints/Health/Health10.Health10"))))

(fn ConstructionScript)

(fn LooseHp
  (params (Value :type Float%20%28single-precision%29))
  (bind _output_get (Variables|Default|SetVie (- (Variables|Default|GetVie) Value)))
  (if (<= _output_get 0.0)
    (Actor|DestroyActor)
    (bind _asmy_camera (Utilities|Casting|CastToMy_Camera (Game|GetPlayerCharacter 0)))
    (Default|AddMoney _asmy_camera 2)
    (bind _asmy_camera_2 (Utilities|Casting|CastToMy_Camera (Game|GetPlayerCharacter 0)))
    (Default|AddScore _asmy_camera_2 1)
    (return false)
    (else
      (return true))))