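; Turret actor that damages AIennemy actors inside its Hitbox and can be upgraded by clicking it.
; An overlap starts a half-second Delay loop that calls LooseHp with Damage while the enemy stays in the Hitbox.
; The loop's stop flag, Life, is one variable shared by all targets and updated from LooseHp's return.
; Clicking the turret spends My_Camera Money to raise Damage, with sound and printed feedback.
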(event OnClicked(Turret)
  (params (TouchedComponent :type Primitive%20Component%20Object%20Reference) (ButtonPressed :type Key%20Structure))
  (bind _asmy_camera (Utilities|Casting|CastToMy_Camera (Game|GetPlayerCharacter 0)))
  (if (>= (Variables|/Game/Game/BluePrints/My_Camera.My_Camera_C|GetMoney _asmy_camera) 15)
    (Audio|PlaySound2D "/Game/Game/Musique/click_constru.click_constru" 0.1 1.0 0.0 0 0)
    (Development|PrintString "Level up! +0,2 damage")
    (Variables|Default|SetDamage (+ (Variables|Default|GetDamage) 0.2))
    (bind _asmy_camera_2 (Utilities|Casting|CastToMy_Camera (Game|GetPlayerCharacter 0)))
    (Variables|/Game/Game/BluePrints/My_Camera.My_Camera_C|SetMoney _asmy_camera_2 (- (Variables|/Game/Game/BluePrints/My_Camera.My_Camera_C|GetMoney _asmy_camera_2) 15))
    (else
      (Audio|PlaySound2D "/Game/Game/Musique/click_menu.click_menu" 0.1 1.0 0.0 0 0)
      (Development|PrintString "Not enought money, need 15"))))

(event Collision|EventActorBeginOverlap
  (params (OtherActor :type Actor%20Object%20Reference))
  (Variables|Default|SetLife true)
  (if (and (Collision|IsOverlappingActor (Variables|Default|GetHitbox) OtherActor :!class /Script/Engine.PrimitiveComponent) (Variables|Default|GetLife)) :!label _label
    (Utilities|FlowControl|Delay 0.5)
    (Utilities|FlowControl|Sequence
      (:then_0
        (bind _asaiennemy (Utilities|Casting|CastToAIennemy OtherActor))
        (bind _life_ (Default|LooseHp _asaiennemy (Variables|Default|GetDamage)))
        (Variables|Default|SetLife _life_))
      (:then_1
        (goto _label)))))

(fn ConstructionScript)